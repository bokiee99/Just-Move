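; Player character for a 2D flipbook runner with Enhanced Input movement, single jump until landing, and a timer-driven survival score.
; Tick picks idle, run, jump or death flipbooks from movement state and IsDead.
; Overlapping a CameraZone switches the detached camera to perspective, animates FOV, unlocks second-axis movement and footstep sounds, and removes music and score HUD.
; PlayerDead shows the game-over widget, then pauses the game.
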(event `EnhancedInput|/Game/2DGAME/IA_2DMOVE`
  (params (ActionValue :type "Vector2D Structure") (ElapsedSeconds :type "Float (double-precision)") (TriggeredSeconds :type "Float (double-precision)") (InputAction :type "InputAction Object Reference" :default "/Game/2DGAME/IA_2DMOVE.IA_2DMOVE"))
  (bind (_x _y) (`KismetMathLibrary.BreakVector2D` ActionValue))
  (:`Triggered`
    (`|ExecutionSequence`
      (:`then_0`
        (if (== _x 1.0)
          (`SceneComponent.SetRelativeScale3D` (`self.Sprite`) (2.0 2.0 2.0))
          (else
            (`SceneComponent.SetRelativeScale3D` (`self.Sprite`) (-2.0 2.0 2.0))))
        (`self.AddMovementInput` (`self.GetActorForwardVector`) _x))
      (:`then_1`
        (if (== _y 1.0)
          (`SceneComponent.SetRelativeScale3D` (`self.Sprite`) (2.0 2.0 2.0)))
        (if (`self.check`)
          (`self.AddMovementInput` (`self.GetActorRightVector`) _y))))))

(event `self.ReceiveBeginPlay`
  (bind _returnvalue (`GameplayStatics.GetPlayerController` 0))
  (`|ExecutionSequence`
    (:`then_0`
      (`KismetSystemLibrary.Delay` 0.01)
      (bind _as2d_move (cast `/Game/2DGAME/2D_Move` (`GameplayStatics.GetPlayerController` 0)))
      (`/Engine/EditorBlueprintResources/StandardMacros.IsValid` _as2d_move
        (:`Is Valid`
          (bind _returnvalue_2 (pcsubsystem `EnhancedInputLocalPlayerSubsystem` _as2d_move))
          (`/Engine/EditorBlueprintResources/StandardMacros.IsValid` _returnvalue_2
            (:`Is Valid`
              (`EnhancedInputSubsystemInterface.AddMappingContext` _returnvalue_2 "/Game/2DGAME/IMC_2D.IMC_2D" 0 (struct)))))))
    (:`then_1`
      (bind _returnvalue_3 (`GameplayStatics.SpawnSoundAtLocation` "/Game/FirstPerson/Sound/2D_BGM_Cue.2D_BGM_Cue" (`self.K2_GetActorLocation` self) (struct) 1.0 1.0 0.0 null null))
      (set `PlayerController.bShowMouseCursor` false _returnvalue)
      (`WidgetBlueprintLibrary.SetInputMode_GameOnly` _returnvalue)
      (`SceneComponent.K2_DetachFromComponent` (`self.Camera`) "KeepWorld" "KeepWorld" "KeepWorld" true)
      (bind _returnvalue_4 (`|CreateWidget` "/Game/2DGAME/Blueprint/BP_ScoreWidget.BP_ScoreWidget_C"))
      (bind _output_get (set `self.Score` _returnvalue_4))
      (`UserWidget.AddToViewport` _output_get 0)
      (`KismetSystemLibrary.K2_SetTimerDelegate` (delegate `Update Score`) 0.1 true))))

(event `Update Score`
  (if (not (`self.IsDead`))
    (bind _result (`/Engine/EditorBlueprintResources/StandardMacros.IncrementInt` (`self.ScoreInt`))
      (:`  `
        (`/Game/2DGAME/Blueprint/BP_ScoreWidget.UpdateScore` (`self.Score`) _result)))))

(event `Key|SpaceBar`
  (params (Key :type "Key Structure"))
  (:`Pressed`
    (if (not (`self.IsDead`))
      (`/Engine/EditorBlueprintResources/StandardMacros.DoOnce` false :!label _label
        (:`Completed`
          (`self.Jump`)
          (`GameplayStatics.PlaySoundAtLocation` "/Game/FirstPerson/Sound/2D-점프_Cue.2D-점프_Cue" (`self.K2_GetActorLocation` self) (struct) 1.0 1.0 0.0 null null null null))))))

(event `self.ReceiveTick`
  (params (DeltaSeconds :type "Float (single-precision)"))
  (bind _charactermovement (`self.CharacterMovement`))
  (if (`self.IsDead`)
    (`PaperFlipbookComponent.SetFlipbook` (`self.Sprite`) "/Game/2DGAME/Astronaut/AstronautDeath.AstronautDeath")
    (`/Engine/EditorBlueprintResources/StandardMacros.IsValid` (stale `self.ReceiveBeginPlay` _returnvalue_3)
      (:`Is Valid`
        (`AudioComponent.Stop` (stale `self.ReceiveBeginPlay` _returnvalue_3))))
    (elif (`NavMovementComponent.IsFalling` _charactermovement)
      (`PaperFlipbookComponent.SetFlipbook` (`self.Sprite`) "/Game/2DGAME/Astronaut/AstronautJump.AstronautJump")
      (elif (> (`KismetMathLibrary.VSize` (`MovementComponent.Velocity` _charactermovement)) 0.0)
        (`PaperFlipbookComponent.SetFlipbook` (`self.Sprite`) "/Game/2DGAME/Astronaut/AstronautRun.AstronautRun")
        (if (`self.checkstep`)
          _
          (elif (`self.bSound`)
            (bind _returnvalue (`GameplayStatics.SpawnSoundAtLocation` (`self.Sound`) (0.0 0.0 0.0) (struct) 1.0 1.0 0.0 null null))
            (set `self.checkstep` true)
            (`KismetSystemLibrary.Delay` 0.2)
            (set `self.checkstep` false)))
        (else
          (`PaperFlipbookComponent.SetFlipbook` (`self.Sprite`) "/Game/2DGAME/Astronaut/Astronaut_Idle1.Astronaut_Idle1")
          (`/Engine/EditorBlueprintResources/StandardMacros.IsValid` _returnvalue
            (:`Is Valid`
              (`AudioComponent.Stop` _returnvalue))))))))

(event `self.OnLanded`
  (params (Hit :type "HitResult Structure (by ref)"))
  (goto _label :!via `Reset`))

(event `self.CapsuleComponent.OnComponentBeginOverlap`
  (params (OverlappedComponent :type "PrimitiveComponent Object Reference") (OtherActor :type "Actor Object Reference") (OtherComp :type "PrimitiveComponent Object Reference") (OtherBodyIndex :type Integer) (bFromSweep :type Boolean) (SweepResult :type "HitResult Structure (by ref)"))
  (cast `/Game/2DGAME/Blueprint/CameraZone` OtherActor)
  (`CameraComponent.SetProjectionMode` (`self.Camera`) "Perspective")
  (set `self.check` true)
  (set `self.bSound` true)
  (set `self.bZone` true)
  (bind (_direction _newtrack_0) (`Timeline|Timeline` :`NewTime` 1.0)
    (:`Update`
      (`CameraComponent.SetFieldOfView` (`self.Camera`) _newtrack_0)
      (`Widget.RemoveFromParent` (stale `self.ReceiveBeginPlay` _returnvalue_4))
      (`/Engine/EditorBlueprintResources/StandardMacros.IsValid` (stale `self.ReceiveBeginPlay` _returnvalue_3)
        (:`Is Valid`
          (`AudioComponent.Stop` (stale `self.ReceiveBeginPlay` _returnvalue_3)))))))

(event `PlayerDead`
  (set `self.IsDead` true)
  (bind _returnvalue (`|CreateWidget` "/Game/2DGAME/Blueprint/BP_GameOver.BP_GameOver_C"))
  (`UserWidget.AddToViewport` _returnvalue 0)
  (`KismetSystemLibrary.Delay` 0.2)
  (`GameplayStatics.SetGamePaused` true))

(fn `UserConstructionScript`)