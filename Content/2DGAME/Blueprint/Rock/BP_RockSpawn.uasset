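; Rock spawner for a 2D game that spawns rock actors at its Scene component's transform, switching rock class as play time passes.
; BeginPlay starts a looping timer with an interval randomized once between half a second and 1.5 seconds.
; Tick accumulates elapsed time, which each timer firing checks to step from BP_Rock through BP_Rock4 every ten seconds, staying on BP_Rock4 thereafter.
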(event `self.ReceiveBeginPlay`
  (`KismetSystemLibrary.K2_SetTimerDelegate` (delegate `Spawn Random Rock`) (`KismetMathLibrary.RandomFloatInRange` 0.5 1.5) true))

(event `Spawn Random Rock`
  (bind _returnvalue (`SceneComponent.K2_GetComponentToWorld` (`self.Scene`)))
  (if (< (`self.TIme`) 10.0)
    (`|SpawnActorFromClass` "/Game/2DGAME/Blueprint/Rock/BP_Rock.BP_Rock_C" _returnvalue "Undefined" "MultiplyWithRoot" null null)
    (elif (< (`self.TIme`) 20.0)
      (`|SpawnActorFromClass` "/Game/2DGAME/Blueprint/Rock/BP_Rock1.BP_Rock1_C" _returnvalue "Undefined" "MultiplyWithRoot" null null)
      (elif (< (`self.TIme`) 30.0)
        (`|SpawnActorFromClass` "/Game/2DGAME/Blueprint/Rock/BP_Rock2.BP_Rock2_C" _returnvalue "Undefined" "MultiplyWithRoot" null null)
        (elif (< (`self.TIme`) 40.0)
          (`|SpawnActorFromClass` "/Game/2DGAME/Blueprint/Rock/BP_Rock3.BP_Rock3_C" _returnvalue "Undefined" "MultiplyWithRoot" null null)
          (elif (< (`self.TIme`) 50.0)
            (`|SpawnActorFromClass` "/Game/2DGAME/Blueprint/Rock/BP_Rock4.BP_Rock4_C" _returnvalue "Undefined" "MultiplyWithRoot" null null)
            (else
              (`|SpawnActorFromClass` "/Game/2DGAME/Blueprint/Rock/BP_Rock4.BP_Rock4_C" _returnvalue "Undefined" "MultiplyWithRoot" null null))))))))

(event `self.ReceiveTick`
  (params (DeltaSeconds :type "Float (single-precision)"))
  (set `self.TIme` (+ DeltaSeconds (`self.TIme`))))

(fn `UserConstructionScript`)