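; Player astronaut character for a 2D flipbook game with a jump action, a time-based score and a game-over state.
; BeginPlay starts music, detaches the camera in world space and creates the score widget, which a looping timer increments while alive.
; Space jumps through a DoOnce reset on landing, while Tick selects the run, jump or death flipbook.
; PlayerDead sets the dead flag, shows the game-over widget and pauses after a short delay.
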(event `self.ReceiveBeginPlay`
  (bind _returnvalue (`GameplayStatics.GetPlayerController` 0))
  (bind _returnvalue_2 (`GameplayStatics.SpawnSoundAtLocation` "/Game/FirstPerson/Sound/2D_BGM_Cue.2D_BGM_Cue" (`self.K2_GetActorLocation` self) (struct) 1.0 1.0 0.0 null null))
  (set `PlayerController.bShowMouseCursor` false _returnvalue)
  (`WidgetBlueprintLibrary.SetInputMode_GameOnly` _returnvalue)
  (`SceneComponent.K2_DetachFromComponent` (`self.Camera`) "KeepWorld" "KeepWorld" "KeepWorld" true)
  (bind _returnvalue_3 (`|CreateWidget` "/Game/2DGAME/Blueprint/BP_ScoreWidget.BP_ScoreWidget_C"))
  (bind _output_get (set `self.Score` _returnvalue_3))
  (`UserWidget.AddToViewport` _output_get 0)
  (`KismetSystemLibrary.K2_SetTimerDelegate` (delegate `Update Score`) 0.1 true))

(event `Update Score`
  (if (not (`self.IsDead`))
    (bind _result (`/Engine/EditorBlueprintResources/StandardMacros.IncrementInt` (`self.ScoreInt`))
      (:`  `
        (`/Game/2DGAME/Blueprint/BP_ScoreWidget.UpdateScore` (`self.Score`) _result)))))

(event `Key|SpaceBar`
  (params (Key :type "Key Structure"))
  (:`Pressed`
    (if (not (`self.IsDead`))
      (`/Engine/EditorBlueprintResources/StandardMacros.DoOnce` false :!label _label
        (:`Completed`
          (`self.Jump`)
          (`GameplayStatics.PlaySoundAtLocation` "/Game/FirstPerson/Sound/2D-점프_Cue.2D-점프_Cue" (`self.K2_GetActorLocation` self) (struct) 1.0 1.0 0.0 null null null null))))))

(event `self.ReceiveTick`
  (params (DeltaSeconds :type "Float (single-precision)"))
  (if (`self.IsDead`)
    (`PaperFlipbookComponent.SetFlipbook` (`self.Sprite`) "/Game/2DGAME/Astronaut/AstronautDeath.AstronautDeath")
    (`/Engine/EditorBlueprintResources/StandardMacros.IsValid` (stale `self.ReceiveBeginPlay` _returnvalue_2)
      (:`Is Valid`
        (`AudioComponent.Stop` (stale `self.ReceiveBeginPlay` _returnvalue_2))))
    (elif (`NavMovementComponent.IsFalling` (`self.CharacterMovement`))
      (`PaperFlipbookComponent.SetFlipbook` (`self.Sprite`) "/Game/2DGAME/Astronaut/AstronautJump.AstronautJump")
      (else
        (`PaperFlipbookComponent.SetFlipbook` (`self.Sprite`) "/Game/2DGAME/Astronaut/AstronautRun.AstronautRun")))))

(event `self.OnLanded`
  (params (Hit :type "HitResult Structure (by ref)"))
  (goto _label :!via `Reset`))

(event `PlayerDead`
  (set `self.IsDead` true)
  (bind _returnvalue (`|CreateWidget` "/Game/2DGAME/Blueprint/BP_GameOver.BP_GameOver_C"))
  (`UserWidget.AddToViewport` _returnvalue 0)
  (`KismetSystemLibrary.Delay` 0.2)
  (`GameplayStatics.SetGamePaused` true))

(fn `UserConstructionScript`)