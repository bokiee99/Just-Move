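; BP_CrossHair is a HUD that draws a crosshair texture while the first-person player has a rifle and is not crouching.
; DrawHUD casts the player pawn and places the texture's top-left corner at screen center, without a half-size offset.
; Otherwise it calls DrawTexture with no texture set.
; The not-crouching check runs in the second Sequence branch, after the condition that uses its result.
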(event `self.ReceiveDrawHUD`
  (params (SizeX :type Integer) (SizeY :type Integer))
  (bind (_x _y) (`KismetMathLibrary.BreakVector2D` (`self.Screen Center`)))
  (set `self.Screen Center` (`KismetMathLibrary.MakeVector2D` (`KismetMathLibrary.Conv_IntToDouble` (/ SizeX 2)) (`KismetMathLibrary.Conv_IntToDouble` (/ SizeY 2))))
  (bind _asbp_first_person_character (cast `/Game/FirstPerson/Blueprints/BP_FirstPersonCharacter` (`GameplayStatics.GetPlayerPawn` 0)))
  (`|ExecutionSequence`
    (:`then_0`
      (bind _returnvalue (`GameCharacter.GetHasRifle` _asbp_first_person_character))
      (if (and _returnvalue (stale _returnvalue_2))
        (`self.DrawTexture` "/Game/Asset/Texture/Cross_Q_9.Cross_Q_9" _x _y 64.0 64.0 0.0 0.0 1.0 1.0)
        (else
          (`self.DrawTexture` null))))
    (:`then_1`
      (bind _returnvalue_2 (`GameCharacter.GetNotCrouching` _asbp_first_person_character)))))

(fn `UserConstructionScript`)